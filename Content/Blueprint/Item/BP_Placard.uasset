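; BP_Placard is an interactable item, apparently a closet, that teleports the interacting player to a paired BP_Placard2.
; On BeginPlay it caches the BP_Placard2 returned by GetActorOfClass, so the link relies on a class lookup.
; Interaction spawns the NS_Clothings Niagara effect at that actor's Arrow, then moves the player to the Arrow's location without changing their rotation.
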(event `self.ReceiveBeginPlay`
  (bind _returnvalue (`GameplayStatics.GetActorOfClass` "/Game/Blueprint/Item/BP_Placard2.BP_Placard2_C"))
  (set `self.NewVar` _returnvalue))

(event `/Game/Blueprint/BPI/BPI_Interact.Interaction`
  (params (PlayerRef :type "/Game/Blueprint/BP_Character Object Reference"))
  (bind _arrow (`/Game/Blueprint/Item/BP_Placard2.Arrow` (`self.NewVar`)))
  (`NiagaraFunctionLibrary.SpawnSystemAtLocation` "/Game/Niagara/NS_Clothings.NS_Clothings" (`SceneComponent.K2_GetComponentLocation` _arrow) (`SceneComponent.K2_GetComponentRotation` _arrow))
  (`self.K2_SetActorLocation` PlayerRef (`SceneComponent.K2_GetComponentLocation` (`/Game/Blueprint/Item/BP_Placard2.Arrow` (`self.NewVar`))) false true))

(fn `UserConstructionScript`)