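; BP_Piege is a single-use trap that stuns any BP_Character entering its box trigger.
; On overlap it sends StunMessage, detaches four cones and launches them as physics bodies in random directions, then destroys the trigger.
; A shared dynamic MI_Dissolve material is applied to the cones, and a timeline animates its DissolveAmount before the actor destroys itself.
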(event `self.Box.OnComponentBeginOverlap`
  (params (OverlappedComponent :type "PrimitiveComponent Object Reference") (OtherActor :type "Actor Object Reference") (OtherComp :type "PrimitiveComponent Object Reference") (OtherBodyIndex :type Integer) (bFromSweep :type Boolean) (SweepResult :type "HitResult Structure (by ref)"))
  (bind _asbp_character (cast `/Game/Blueprint/BP_Character` OtherActor))
  (message `/Game/Blueprint/BPI/BPI_Hit.Stun` _asbp_character 3.0)
  (for _array_element (`|MakeArray` (`self.Cone`) (`self.Cone2`) (`self.Cone3`) (`self.Cone1`))
    (`SceneComponent.K2_DetachFromComponent` _array_element "KeepWorld" "KeepWorld" "KeepRelative" true)
    (`PrimitiveComponent.SetSimulatePhysics` _array_element true)
    (`PrimitiveComponent.SetPhysicsLinearVelocity` _array_element (* (`KismetMathLibrary.RandomUnitVector`) 1500.0) true "None"))
  (`ActorComponent.K2_DestroyComponent` (`self.Box`))
  (bind _returnvalue (`KismetMaterialLibrary.CreateDynamicMaterialInstance` "/Game/Material/MI_Dissolve.MI_Dissolve"))
  (set `self.DissolveRef` _returnvalue)
  (`PrimitiveComponent.SetMaterial` (`self.Cone1`) 0 _returnvalue)
  (`PrimitiveComponent.SetMaterial` (`self.Cone`) 0 _returnvalue)
  (`PrimitiveComponent.SetMaterial` (`self.Cone2`) 0 _returnvalue)
  (`PrimitiveComponent.SetMaterial` (`self.Cone3`) 0 _returnvalue)
  (bind (_direction _alpha) (`Timeline|DisolveTimeline` :!via `PlayFromStart`)
    (:`Update`
      (`MaterialInstanceDynamic.SetScalarParameterValue` (`self.DissolveRef`) "DissolveAmount" _alpha))
    (:`Finished`
      (`self.K2_DestroyActor`))))

(fn `UserConstructionScript`)