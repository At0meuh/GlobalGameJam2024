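; Clown-themed weapon item whose Shoot event either pops out flowers or honks a horn, depending on IsWeapon.
; As a weapon, it plays the FlowersScale timeline to grow the Flowers component from zero to half scale.
; A ReverseR flag toggled on timeline completion decides when Reverse plays it backwards to shrink them.
; Otherwise, it plays a honk sound and spawns the Klaxon Niagara effect at the Arrow.
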(event `Shoot`
  (bind _arrow (`self.Arrow`))
  (if (`self.IsWeapon`)
    (bind (_direction _scale) (`Timeline|FlowersScale` :!via `PlayFromStart` :!label _label)
      (:`Update`
        (`SceneComponent.SetRelativeScale3D` (`self.Flowers`) (`KismetMathLibrary.VLerp` (0.0 0.0 0.0) (0.5 0.5 0.5) _scale)))
      (:`Finished`
        (if (`self.ReverseR`)
          (`self.Reverse`)
          (set `self.ReverseR` false)
          (else
            (set `self.ReverseR` true)))))
    (else
      (`GameplayStatics.PlaySound2D` "/Game/Sounds/Clown_Honk_Sound_Effect__Free_Download___No_Copyright_.Clown_Honk_Sound_Effect__Free_Download___No_Copyright_" 1.0 1.0 0.0 null null)
      (`NiagaraFunctionLibrary.SpawnSystemAtLocation` "/Game/Niagara/NS_Klaxon.NS_Klaxon" (`SceneComponent.K2_GetComponentLocation` _arrow) (`SceneComponent.K2_GetComponentRotation` _arrow)))))

(event `Reverse`
  (set `self.ReverseR` false)
  (goto _label :!via `ReverseFromEnd`))

(fn `UserConstructionScript`
  (`parent.UserConstructionScript`))