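; Item spawner that places random principal items at its own transform, drawn from the ItemP pool on RefMaster.
; On BeginPlay a 90% roll gates both the spawn and a 20-second looping timer, which re-enters the same roll.
; A failed first roll leaves the spawner idle.
; Each spawn also removes a randomly picked entry from the pool, evaluated separately, so it can differ from the spawned item.
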(event `self.ReceiveBeginPlay`
  (if (`KismetMathLibrary.RandomBoolWithWeight` 0.9) :!label _label
    (`self.SpawnPrincipalItems`)
    (`KismetSystemLibrary.K2_SetTimerDelegate` (delegate `suiiiiiiiii`) 20.0 true)))

(event `suiiiiiiiii`
  (goto _label))

(fn `SpawnPrincipalItems`
  (bind _itemp (`/Game/Blueprint/Item/BP_ItemSpawnerMaster.ItemP` (`self.RefMaster`)))
  (bind _outitem (`KismetArrayLibrary.Array_Random` _itemp))
  (`|SpawnActorFromClass` _outitem (`self.GetTransform`) "Undefined" "MultiplyWithRoot" null null)
  (`KismetArrayLibrary.Array_RemoveItem` _itemp _outitem))

(fn `UserConstructionScript`)