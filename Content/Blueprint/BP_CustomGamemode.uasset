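; Custom game mode that sets up two local players when play begins, each controlling its own BP_Character.
; BeginPlay loops over both player indices, calls CreatePlayer and adds the IMC_Default Enhanced Input mapping context to each player's subsystem.
; It then spawns a character at a hard-coded location per player and possesses it, with the first player handled through the existing controller 0.
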(event `self.ReceiveBeginPlay`
  (bind _returnvalue (`GameplayStatics.GetPlayerController` 0))
  (for _index (range 2)
    (bind _returnvalue_2 (`GameplayStatics.CreatePlayer` _index))
    (if (> _index 0)
      (`EnhancedInputSubsystemInterface.AddMappingContext` (pcsubsystem `EnhancedInputLocalPlayerSubsystem` _returnvalue_2) "/Game/Blueprint/Input/IMC_Default.IMC_Default" 0 (struct))
      (bind _returnvalue_3 (`|SpawnActorFromClass` "/Game/Blueprint/BP_Character.BP_Character_C" (`KismetMathLibrary.MakeTransform` (500.0 500.0 0.0)) "Undefined" "MultiplyWithRoot" null null))
      (`Controller.Possess` (`GameplayStatics.GetPlayerController` _index) _returnvalue_3)
      (else
        (`EnhancedInputSubsystemInterface.AddMappingContext` (pcsubsystem `EnhancedInputLocalPlayerSubsystem` _returnvalue) "/Game/Blueprint/Input/IMC_Default.IMC_Default" 0 (struct))
        (bind _returnvalue_4 (`|SpawnActorFromClass` "/Game/Blueprint/BP_Character.BP_Character_C" (`KismetMathLibrary.MakeTransform` (700.0 700.0 0.0)) "Undefined" "MultiplyWithRoot" null null))
        (`Controller.Possess` _returnvalue _returnvalue_4)))))

(fn `UserConstructionScript`)