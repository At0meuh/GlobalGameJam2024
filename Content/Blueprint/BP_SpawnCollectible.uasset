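; Spawner actor that scatters a random batch of BP_Collectible actors inside its Box bounds when SpawnCollectible is called.
; It first plays one of two Niagara effects chosen by the player's LaughGuys flag, then waits briefly before spawning.
; Each collectible gets a random X/Y in the box at the passed actor's height.
; Each also receives the LaughGuys flag and the BP_Child reference cached at BeginPlay.
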(event `self.ReceiveBeginPlay`
  (bind _returnvalue (`GameplayStatics.GetActorOfClass` "/Game/Blueprint/BP_Child.BP_Child_C"))
  (set `self.Ref_Child` _returnvalue))

(event `/Game/Blueprint/BPI/BPI_SpawnCollectible.spawnCollectible`
  (params (PlayerRef :type "/Game/Blueprint/BP_Character Object Reference") (ActorRef :type "Actor Object Reference"))
  (bind (_returnvalue_x _returnvalue_y _returnvalue_z) (`KismetMathLibrary.BreakVector` (`self.K2_GetActorLocation` ActorRef)))
  (bind (_origin _boxextent) (`KismetSystemLibrary.GetComponentBounds` (`self.Box`)))
  (bind (_returnvalue_x_2 _returnvalue_y_2) (`KismetMathLibrary.BreakVector` (`KismetMathLibrary.RandomPointInBoundingBox` _origin _boxextent)))
  (`NiagaraFunctionLibrary.SpawnSystemAtLocation` (select `bool` (`/Game/Blueprint/BP_Character.LaughGuys?` PlayerRef) :`false` "/Game/Niagara/NS_Clothings.NS_Clothings" :`true` "/Game/Niagara/NS_Collectible.NS_Collectible" :!type "NiagaraSystem Object Reference") (`self.K2_GetActorLocation`))
  (`KismetSystemLibrary.Delay` 1.35)
  (for _ (range (+ (`KismetMathLibrary.RandomIntegerInRange` 4 10) 1))
    (`|SpawnActorFromClass` "/Game/Blueprint/BP_Collectible.BP_Collectible_C" (`KismetMathLibrary.MakeTransform` (`KismetMathLibrary.MakeVector` _returnvalue_x_2 _returnvalue_y_2 _returnvalue_z)) "Undefined" "MultiplyWithRoot" null (`/Game/Blueprint/BP_Character.LaughGuys?` PlayerRef) (`self.Ref_Child`) null)))

(fn `UserConstructionScript`)