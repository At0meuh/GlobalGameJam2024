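; Game mode, named for the main menu, that sets up a shared camera and judges a timed match from the child's Happiness.
; BeginPlay spawns and views through BP_Camera, caches the child, game instance and widget manager, and creates the end-game widget.
; PlayGameTimer starts the countdown; on expiry, Happiness against a midpoint awards player 0, player 1 or both, then shows the end screen.
; An unconnected chain for spawning two local players never runs.
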(event `PlayGameTimer`
  (bind _returnvalue (`KismetSystemLibrary.K2_SetTimerDelegate` (delegate `FinDuTimer`) (`self.TimeForAGame`)))
  (set `self.Timer` _returnvalue))

(event `FinDuTimer`
  (bind _gameinsatanceref (`self.GameInsatanceRef`))
  (bind _happiness (`/Game/Blueprint/BP_Child.happiness` (`self.ChildRef`)))
  (if (== _happiness 5000.0)
    (`/Game/Blueprint/BP_CustomGameInstance.AddToWin` _gameinsatanceref 0)
    (`/Game/Blueprint/BP_CustomGameInstance.AddToWin` _gameinsatanceref 1)
    (else
      (`/Game/Blueprint/BP_CustomGameInstance.AddToWin` _gameinsatanceref (`KismetMathLibrary.SelectInt` 1 0 (< _happiness 5000.0)))))
  ;[1 1 1] Comment
  (`/Game/Blueprint/BP_WidgetManager.ShowEndGame` (`self.WidgetManagerRef`)))

(event `self.ReceiveBeginPlay`
  (`|ExecutionSequence`
    (:`then_1`
      (bind _returnvalue (`|SpawnActorFromClass` "/Game/Blueprint/Camera/BP_Camera.BP_Camera_C" (`KismetMathLibrary.MakeTransform` (0.0 0.0 0.0) (struct :`Yaw` 180.0)) "Undefined" "MultiplyWithRoot" null (`self.PlayerRef`) null))
      (set `self.Ref_Camera` _returnvalue)
      (`PlayerController.SetViewTargetWithBlend` (`GameplayStatics.GetPlayerController` 0) _returnvalue 0.0 "VTBlend_Linear" 0.0 false))
    (:`then_2`
      (bind _returnvalue_2 (`GameplayStatics.GetActorOfClass` "/Game/Blueprint/BP_Child.BP_Child_C"))
      (set `self.ChildRef` _returnvalue_2)
      (set `self.GameInsatanceRef` (cast `/Game/Blueprint/BP_CustomGameInstance` (`GameplayStatics.GetGameInstance`) :!pure true))
      (bind _returnvalue_3 (`GameplayStatics.GetActorOfClass` "/Game/Blueprint/BP_WidgetManager.BP_WidgetManager_C"))
      (bind _output_get (set `self.WidgetManagerRef` _returnvalue_3))
      (`/Game/Blueprint/BP_WidgetManager.CreateEndGame` _output_get 0))))

(fn `UserConstructionScript`)