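; BP_Collectible is a spinning, bobbing pickup that adds points to the child's Happiness, with its Laugh flag selecting the material at construction.
; A timeline drives idle motion until a character with matching Laugh state enters the Box, then homing projectile movement pulls the item toward that character's mesh.
; Overlap on AddToScore by a matching character plays force feedback for that player, updates Happiness and the HUD, then destroys the item.
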(event `self.ReceiveBeginPlay`
  (bind _initlocation (`self.InitLocation`))
  (set `self.InitLocation` (`self.K2_GetActorLocation`))
  (bind (_direction _alpha) (`Timeline|SmouthRotate` :!via `PlayFromStart`)
    (:`Update`
      (`self.K2_AddActorWorldRotation` (struct :`Yaw` 0.6))
      (`self.K2_SetActorLocation` (`KismetMathLibrary.VLerp` _initlocation (+ _initlocation (0.0 0.0 50.0)) _alpha)))))

(event `self.Box.OnComponentBeginOverlap`
  (params (OverlappedComponent :type "PrimitiveComponent Object Reference") (OtherActor :type "Actor Object Reference") (OtherComp :type "PrimitiveComponent Object Reference") (OtherBodyIndex :type Integer) (bFromSweep :type Boolean) (SweepResult :type "HitResult Structure (by ref)"))
  (bind _projectilemovement (`self.ProjectileMovement`))
  (bind _asbp_character (cast `/Game/Blueprint/BP_Character` OtherActor))
  (if (== (`/Game/Blueprint/BP_Character.LaughGuys?` _asbp_character) (`self.Laugh?`))
    (`TimelineComponent.Stop` (`self.SmouthRotate`))
    (set `ProjectileMovementComponent.bIsHomingProjectile` true _projectilemovement)
    (set `ProjectileMovementComponent.HomingTargetComponent` (`Character.Mesh` _asbp_character) _projectilemovement)
    (`ActorComponent.Activate` _projectilemovement false)))

(event `self.AddToScore.OnComponentBeginOverlap`
  (params (OverlappedComponent :type "PrimitiveComponent Object Reference") (OtherActor :type "Actor Object Reference") (OtherComp :type "PrimitiveComponent Object Reference") (OtherBodyIndex :type Integer) (bFromSweep :type Boolean) (SweepResult :type "HitResult Structure (by ref)"))
  (bind _bp_childref (`self.Bp_ChildRef`))
  (bind _asbp_character (cast `/Game/Blueprint/BP_Character` OtherActor))
  (if (== (`/Game/Blueprint/BP_Character.LaughGuys?` _asbp_character) (`self.Laugh?`))
    (`PlayerController.K2_ClientPlayForceFeedback` (`GameplayStatics.GetPlayerController` (`/Game/Blueprint/BP_Character.IdPlayer` _asbp_character)) "/Game/Haptique/FB_GetItem.FB_GetItem" "None" false false false)
    (bind _output_get (set `/Game/Blueprint/BP_Child.happiness` (+ (`/Game/Blueprint/BP_Child.happiness` _bp_childref) (`self.PointsToAdd`)) _bp_childref))
    (`/Game/Widget/HUD/WBP_HUD.HandleHapiness` (`/Game/Blueprint/BP_WidgetManager.WBP_HUD_Ref` (`/Game/Blueprint/BP_Child.WidgetManagerRef` _bp_childref)) _output_get)
    (`self.K2_DestroyActor`)))

(fn `UserConstructionScript`
  (bind _plane (`self.Plane`))
  (if (`self.Laugh?`)
    (`PrimitiveComponent.SetMaterial` _plane 0 "/Game/Material/M_Points.M_Points")
    (else
      (`PrimitiveComponent.SetMaterial` _plane 0 "/Game/Material/MI_Bouh.MI_Bouh"))))