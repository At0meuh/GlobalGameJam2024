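; BP_Child is a child actor that the player gives held items to in order to raise its Happiness.
; A box overlap flags BP_Character as near the child and stores a reference to it.
; While flagged, Interaction calls the player's Batet, spawns a collectible message, adds the item's ScoreLaugh, destroys the item and notifies the HUD.
; Tick prints Happiness on screen every frame.
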(event `self.ReceiveTick`
  (params (DeltaSeconds :type "Float (single-precision)"))
  (`KismetSystemLibrary.PrintString` (`KismetStringLibrary.Conv_DoubleToString` (`self.happiness`)) true true (struct :`G` 0.66 :`B` 1.0 :`A` 1.0) 0.0))

(event `self.Box.OnComponentBeginOverlap`
  (params (OverlappedComponent :type "PrimitiveComponent Object Reference") (OtherActor :type "Actor Object Reference") (OtherComp :type "PrimitiveComponent Object Reference") (OtherBodyIndex :type Integer) (bFromSweep :type Boolean) (SweepResult :type "HitResult Structure (by ref)"))
  (bind _asbp_character (cast `/Game/Blueprint/BP_Character` OtherActor))
  (set `/Game/Blueprint/BP_Character.IsInChild?` true _asbp_character)
  (set `/Game/Blueprint/BP_Character.ChildRef` self _asbp_character))

(event `self.Box.OnComponentEndOverlap`
  (params (OverlappedComponent :type "PrimitiveComponent Object Reference") (OtherActor :type "Actor Object Reference") (OtherComp :type "PrimitiveComponent Object Reference") (OtherBodyIndex :type Integer))
  (bind _asbp_character (cast `/Game/Blueprint/BP_Character` OtherActor))
  (set `/Game/Blueprint/BP_Character.IsInChild?` false _asbp_character))

(event `self.ReceiveBeginPlay`)

(event `/Game/Blueprint/BPI/BPI_Interact.Interaction`
  (params (PlayerRef :type "/Game/Blueprint/BP_Character Object Reference"))
  (bind (_s_item_association _s_item_typeitem _s_item_aceesplace _s_item_scorelaugh) (break `/Game/Blueprint/Item/S_Item` (`/Game/Blueprint/Item/Bp_ItemMain.S_Item` (`/Game/Blueprint/BP_Character.ItemInHand` PlayerRef))))
  (if (`/Game/Blueprint/BP_Character.IsInChild?` PlayerRef)
    (`/Game/Blueprint/BP_Character.Batet` PlayerRef)
    (message `/Game/Blueprint/BPI/BPI_SpawnCollectible.spawnCollectible` (`self.ActorRef`) PlayerRef self)
    (set `self.happiness` (+ (`self.happiness`) _s_item_scorelaugh))
    (`self.K2_DestroyActor` (`/Game/Blueprint/BP_Character.ItemInHand` PlayerRef))
    (set `/Game/Blueprint/BP_Character.ItemInHand` null PlayerRef)
    (`/Game/Widget/HUD/WBP_HUD.HandleHapiness` (`/Game/Blueprint/BP_WidgetManager.WBP_HUD_Ref` (`self.WidgetManagerRef`)) 0.0)))

(fn `UserConstructionScript`)