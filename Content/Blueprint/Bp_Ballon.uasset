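; Throwable ball actor that a player picks up, carries and launches to kill other characters.
; Interaction freezes the player's walking and snaps the physics sphere to their mesh socket; Release restores movement and launches it along their forward vector.
; While held and for two seconds after release, box overlaps send KillMessage to any BP_Character except the launcher.
; When destroyed, it spawns a replacement of itself.
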(event `/Game/Blueprint/BPI/BPI_Interact.Interaction`
  (params (PlayerRef :type "/Game/Blueprint/BP_Character Object Reference"))
  (bind _sphere1 (`self.Sphere1`))
  (if (not (`self.Activate`))
    (set `self.LauncherRef` PlayerRef)
    (set `self.Activate` true)
    (set `CharacterMovementComponent.MaxWalkSpeed` 0.0 (`Character.CharacterMovement` PlayerRef))
    (`PrimitiveComponent.SetSimulatePhysics` _sphere1 false)
    (`self.K2_AttachToComponent` (`Character.Mesh` PlayerRef) "Attach" "SnapToTarget" "SnapToTarget" "KeepWorld")
    (`PrimitiveComponent.SetCollisionEnabled` _sphere1 "NoCollision")
    (`PrimitiveComponent.SetPhysicsLinearVelocity` (`self.Sphere1`) (0.0 0.0 0.0) false "None")))

(event `/Game/Blueprint/BPI/BPI_Release.Release`
  (params (PlayerRef :type "/Game/Blueprint/BP_Character Object Reference"))
  (bind _sphere1 (`self.Sphere1`))
  (if (`self.Activate`)
    (`KismetSystemLibrary.K2_SetTimerDelegate` (delegate `ResetActivation`) 2.0)
    (set `CharacterMovementComponent.MaxWalkSpeed` 500.0 (`Character.CharacterMovement` PlayerRef))
    (`PrimitiveComponent.SetCollisionEnabled` (`self.Sphere1`) "QueryAndPhysics")
    (`PrimitiveComponent.SetSimulatePhysics` _sphere1 true)
    (`SceneComponent.K2_DetachFromComponent` _sphere1 "KeepWorld" "KeepWorld" "KeepWorld" true)
    (`PrimitiveComponent.SetPhysicsLinearVelocity` (`self.Sphere1`) (* (`self.GetActorForwardVector` PlayerRef) 1500.0) false "None")))

(event `ResetActivation`
  (set `self.Activate` false)
  (set `self.LauncherRef` null))

(event `self.ReceiveBeginPlay`
  (add `self.OnDestroyed` (delegate `OnDestroyed_Event`)))

(event `OnDestroyed_Event` :!signature `self.OnDestroyed`
  (params (DestroyedActor :type "Actor Object Reference"))
  (`KismetSystemLibrary.PrintString` "Hello")
  (`|SpawnActorFromClass` "Bp_Ballon_C" (`KismetMathLibrary.MakeTransform` (`self.Spawn Transform Location`)) "Undefined" "MultiplyWithRoot" null null))

(event `self.Box.OnComponentBeginOverlap`
  (params (OverlappedComponent :type "PrimitiveComponent Object Reference") (OtherActor :type "Actor Object Reference") (OtherComp :type "PrimitiveComponent Object Reference") (OtherBodyIndex :type Integer) (bFromSweep :type Boolean) (SweepResult :type "HitResult Structure (by ref)"))
  (bind _asbp_character (cast `/Game/Blueprint/BP_Character` OtherActor))
  (`/Engine/EditorBlueprintResources/StandardMacros.IsValid` (`self.LauncherRef`)
    (:`Is Valid`
      (if (and (`self.Activate`) (not (== _asbp_character (`self.LauncherRef`))))
        (message `/Game/Blueprint/BPI/BPI_Hit.Kill` _asbp_character)))))

(fn `UserConstructionScript`)