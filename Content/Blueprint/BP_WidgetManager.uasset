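; Widget manager Blueprint that creates and displays the game's main menu, HUD, end-game and loading screen widgets.
; BeginPlay caches BP_CustomGamemode for the HUD, and separate custom events build each widget and store its reference.
; HUD and end-game split creation from validity-checked display, with SpawnHUD chaining both HUD steps.
; The main menu sets UI-only input with the cursor hidden, and it and the loading screen receive a manager reference.
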(event `self.ReceiveBeginPlay`
  (bind _asbp_custom_gamemode (cast `/Game/Blueprint/BP_CustomGamemode` (`GameplayStatics.GetGameMode`))
    (:`then`
      (set `self.GamemoedRef` _asbp_custom_gamemode))
    (:`CastFailed`
      (`KismetSystemLibrary.PrintString` "custom gamemode cast fail widget manager"))))

(event `EventBegin`
  (bind _returnvalue (`GameplayStatics.GetPlayerController` 0))
  (bind _returnvalue_2 (`|CreateWidget` "/Game/Widget/MainMenu/WBP_MainMenu.WBP_MainMenu_C" null self))
  (bind _output_get (set `self.WBP_MainMenuRef` _returnvalue_2))
  (`UserWidget.AddToViewport` _output_get 0)
  (`WidgetBlueprintLibrary.SetInputMode_UIOnlyEx` _returnvalue _output_get)
  (set `PlayerController.bShowMouseCursor` false _returnvalue))

(event `CreateWBP_HUD`
  (bind _returnvalue (`|CreateWidget` "/Game/Widget/HUD/WBP_HUD.WBP_HUD_C" null (`self.GamemoedRef`)))
  (set `self.WBP_HUD_Ref` _returnvalue))

(event `ShowWBP_HUD`
  (bind _wbp_hud_ref (`self.WBP_HUD_Ref`)
    (:`then`
      (`UserWidget.AddToViewport` _wbp_hud_ref 0))
    (:`else`)))

(event `CreateEndGame`
  (bind _returnvalue (`|CreateWidget` "/Game/Widget/EndGame/WBP_EndGame.WBP_EndGame_C" null null))
  (set `self.WBP_EndGameREf` _returnvalue))

(event `ShowEndGame`
  (bind _wbp_endgameref (`self.WBP_EndGameREf`)
    (:`then`
      (`UserWidget.AddToViewport` _wbp_endgameref 0))
    (:`else`)))

(event `SpawnHUD`
  (`self.CreateWBP_HUD`)
  (`self.ShowWBP_HUD`))

(event `LoadingScreen`
  (bind _returnvalue (`|CreateWidget` "/Game/Widget/loadingScreen/WBP_loadingScreen.WBP_loadingScreen_C" null self))
  (bind _output_get (set `self.LoadingScreenRef` _returnvalue))
  (`UserWidget.AddToViewport` _output_get 0)
  (`UserWidget.AddToViewport` _returnvalue 0))

(fn `UserConstructionScript`)