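; BP_Armoire is an interactable armoire that hands out a weapon after a short random delay.
; A timer starts a light-intensity timeline that sets IsItem, which unlocks Interaction and is never cleared.
; Interactions then alternate through a FlipFlop: opening spawns BP_Weapon along the Cube-to-Cube1 direction with a Niagara effect, rotates the Pivot and turns the light off.
; Closing reverses the rotation and restarts the timer.
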(event `self.ReceiveBeginPlay`
  (`KismetSystemLibrary.K2_SetTimerDelegate` (delegate `Item`) (`KismetMathLibrary.RandomFloatInRange` 1.0 3.0) :!label _label))

(event `RestartTimer`
  (goto _label))

(event `Item`
  (bind (_direction _newtrack_0) (`Timeline|Timeline_0` :!via `PlayFromStart`)
    (:`Update`
      (`LightComponent.SetIntensity` (`self.PointLight`) (`KismetMathLibrary.Lerp` 5000.0 500.0 _newtrack_0))
      (set `self.IsItem?` true))))

(event `/Game/Blueprint/BPI/BPI_Interact.Interaction`
  (params (PlayerRef :type "/Game/Blueprint/BP_Character Object Reference"))
  (if (`self.IsItem?`)
    (`/Engine/EditorBlueprintResources/StandardMacros.FlipFlop`
      (:`A`
        (`|SpawnActorFromClass` "/Game/Blueprint/Item/ItemChild/LaughGuys/BP_Weapon.BP_Weapon_C" (`KismetMathLibrary.MakeTransform` (+ (`self.K2_GetActorLocation`) (* (`KismetMathLibrary.Normal` (- (`SceneComponent.K2_GetComponentLocation` (`self.Cube1`)) (`SceneComponent.K2_GetComponentLocation` (`self.Cube`)))) 200.0))) "Undefined" "MultiplyWithRoot" null null)
        (`NiagaraFunctionLibrary.SpawnSystemAtLocation` "/Game/Niagara/NS_OpenArmoire.NS_OpenArmoire" (`SceneComponent.K2_GetComponentLocation` (`self.Scene`)) (struct) (2.0 2.0 2.0))
        (bind (_direction _alpha) (`Timeline|Timeline` :!label _label_2)
          (:`Update`
            (`SceneComponent.K2_SetRelativeRotation` (`self.Pivot`) (`KismetMathLibrary.RLerp` (struct) (struct :`Yaw` 90.0) _alpha) false false))
          (:`Finished`
            (`LightComponent.SetIntensity` (`self.PointLight`) 0.0))))
      (:`B`
        (`self.RestartTimer`)
        (`TimelineComponent.Stop` (`self.Timeline_0`))
        (goto _label_2 :!via `Reverse`)))))

(fn `UserConstructionScript`)