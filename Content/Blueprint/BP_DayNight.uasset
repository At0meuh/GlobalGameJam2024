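; BP_DayNight is a day/night lighting actor that animates a directional light over time.
; A slowed timeline starts on BeginPlay, interpolating the actor's rotation between two fixed orientations and the light intensity through a separate alpha track.
; The GoNight event restarts that same timeline from the beginning.
; The construction script sets the actor to the starting orientation.
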(event `self.ReceiveBeginPlay`
  (`TimelineComponent.SetPlayRate` (`self.DayNight`) (/ 1.0 10.0) :!label _label)
  (bind (_direction _alpha _alphaintensity) (`Timeline|DayNight` :!via `PlayFromStart`)
    (:`Update`
      (`self.K2_SetActorRotation` (`KismetMathLibrary.RLerp` (struct :`Pitch` -40.0 :`Yaw` -90.0) (struct :`Pitch` -40.0 :`Yaw` -270.0) _alpha))
      (`LightComponent.SetIntensity` (`self.DirectionalLight`) (`KismetMathLibrary.Lerp` 0.1 0.7 _alphaintensity)))))

(event `GoNight`
  (goto _label))

(fn `UserConstructionScript`
  (`self.K2_SetActorRotation` (struct :`Pitch` -40.0 :`Yaw` -90.0)))