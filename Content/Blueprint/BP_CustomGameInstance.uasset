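; Custom game instance that keeps the round-win score for a two-player match and ends the match when a player reaches three wins.
; AddToWin increments the counter selected by the winner's index, then at the threshold shows the WBP_EndGame widget and pauses the game.
; ResetVariable zeroes both counters, and the Init event is empty.
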(event `self.ReceiveInit`)

(fn `AddToWin`
  (params (IdPlayerWin :type Integer))
  (locals (IndexLocal :type Integer))
  (bind _output_get (set `local.IndexLocal` IdPlayerWin))
  (bind _result (`/Engine/EditorBlueprintResources/StandardMacros.IncrementInt` (select `int` _output_get :`0` (`self.RoundPlayer 1`) :`1` (`self.RoundPlayer 2`)))
    (:`  `
      (if (>= _result 3)
        (bind _returnvalue (`|CreateWidget` "/Game/Widget/EndGame/WBP_EndGame.WBP_EndGame_C" null null))
        (`UserWidget.AddToViewport` _returnvalue 0)
        (`GameplayStatics.SetGamePaused` true)))))

(fn `ResetVariable`
  (set `self.RoundPlayer 1` 0)
  (set `self.RoundPlayer 2` 0))